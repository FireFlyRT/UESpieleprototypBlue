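; Player-controlled villager pawn that handles Enhanced Input for movement, look, jump, magic zones, item handling and a timed punch.
; CCharacterController tracks right-hand items, receiving pickups from camera line traces of tagged objects, plus drops.
; Placing spawns a physics-handle preview of the held mesh that follows the camera, rotates by modifier keys, and transfers its transform to the item on release.
; Punching briefly enables a hand-socket collision alongside the animation.
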(event `self.ReceiveBeginPlay`
  (bind _rightpunchcollision (`self.RightPunchCollision`))
  (bind _asplayer_controller (cast `PlayerController` (`self.GetController`)))
  (message `EnhancedInputSubsystemInterface.AddMappingContext` (pcsubsystem `EnhancedInputLocalPlayerSubsystem` _asplayer_controller) "/Game/Input/PlayerVillagerInput.PlayerVillagerInput" 0 (struct))
  (`SceneComponent.K2_AttachToComponent` _rightpunchcollision (`self.Mesh`) "hand_rSocket" "SnapToTarget" "SnapToTarget" "SnapToTarget" true)
  (`PrimitiveComponent.SetCollisionEnabled` _rightpunchcollision "NoCollision"))

(event `EnhancedInput|/Game/Input/PlayerMovement`
  (params (ActionValue :type "Vector2D Structure") (ElapsedSeconds :type "Float (double-precision)") (TriggeredSeconds :type "Float (double-precision)") (InputAction :type "InputAction Object Reference" :default "/Game/Input/PlayerMovement.PlayerMovement"))
  (bind (_x _y) (`KismetMathLibrary.BreakVector2D` ActionValue))
  (bind _returnvalue (`SceneComponent.K2_GetComponentRotation` (`self.Mesh`)))
  (:`Triggered`
    (bind _result (`/Engine/EditorBlueprintResources/StandardMacros.NegateFloat` _x)
      (:`  `
        (`self.AddMovementInput` (`KismetMathLibrary.GetForwardVector` _returnvalue) _result)
        (`self.AddMovementInput` (`KismetMathLibrary.GetRightVector` _returnvalue) _y)))))

(event `EnhancedInput|/Game/Input/PlayerLook`
  (params (ActionValue :type "Vector2D Structure") (ElapsedSeconds :type "Float (double-precision)") (TriggeredSeconds :type "Float (double-precision)") (InputAction :type "InputAction Object Reference" :default "/Game/Input/PlayerLook.PlayerLook"))
  (:`Triggered`
    (`CCharacterController.OnLook` (`self.CCharacterController`) (`KismetMathLibrary.Conv_Vector2DToVector` ActionValue))))

(event `EnhancedInput|/Game/Input/PlayerCreateMagicZone`
  (params (ActionValue :type Boolean) (ElapsedSeconds :type "Float (double-precision)") (TriggeredSeconds :type "Float (double-precision)") (InputAction :type "InputAction Object Reference" :default "/Game/Input/PlayerCreateMagicZone.PlayerCreateMagicZone"))
  (:`Triggered`
    (`CCharacterController.CreateMagicZone` (`self.CCharacterController`) (`self.GetTransform`) (`self.GetActorForwardVector`))))

(event `EnhancedInput|/Game/Input/PlayerAcceptMagicZone`
  (params (ActionValue :type Boolean) (ElapsedSeconds :type "Float (double-precision)") (TriggeredSeconds :type "Float (double-precision)") (InputAction :type "InputAction Object Reference" :default "/Game/Input/PlayerAcceptMagicZone.PlayerAcceptMagicZone"))
  (:`Triggered`
    (`CCharacterController.AcceptMagicZone` (`self.CCharacterController`))))

(event `EnhancedInput|/Game/Input/ShiftActive`
  (params (ActionValue :type Boolean) (ElapsedSeconds :type "Float (double-precision)") (TriggeredSeconds :type "Float (double-precision)") (InputAction :type "InputAction Object Reference" :default "/Game/Input/ShiftActive.ShiftActive"))
  (:`Started`
    (set `self.IsShiftActive` true))
  (:`Completed`
    (set `self.IsShiftActive` false)))

(event `EnhancedInput|/Game/Input/StrgActive`
  (params (ActionValue :type Boolean) (ElapsedSeconds :type "Float (double-precision)") (TriggeredSeconds :type "Float (double-precision)") (InputAction :type "InputAction Object Reference" :default "/Game/Input/StrgActive.StrgActive"))
  (:`Started`
    (set `self.IsStrgActive` true))
  (:`Completed`
    (set `self.IsStrgActive` false)))

(event `EnhancedInput|/Game/Input/PlayerJump`
  (params (ActionValue :type Boolean) (ElapsedSeconds :type "Float (double-precision)") (TriggeredSeconds :type "Float (double-precision)") (InputAction :type "InputAction Object Reference" :default "/Game/Input/PlayerJump.PlayerJump"))
  (:`Started`
    (`self.Jump`)))

(event `EnhancedInput|/Game/Input/PlayerPickUp`
  (params (ActionValue :type Boolean) (ElapsedSeconds :type "Float (double-precision)") (TriggeredSeconds :type "Float (double-precision)") (InputAction :type "InputAction Object Reference" :default "/Game/Input/PlayerPickUp.PlayerPickUp"))
  (bind _ccharactercontroller (`self.CCharacterController`))
  (bind _camera (`self.Camera`))
  (bind _returnvalue (`SceneComponent.K2_GetComponentLocation` _camera))
  (:`Started`
    (bind _outhit (`KismetSystemLibrary.LineTraceSingle` :`Start` _returnvalue :`End` (+ _returnvalue (* (`SceneComponent.GetForwardVector` _camera) 1024.0)) :`TraceChannel` "TraceTypeQuery1" :`DrawDebugType` "ForDuration" :`DrawTime` 3.0))
    (bind (_bblockinghit _binitialoverlap _time _distance _location _impactpoint _normal _impactnormal _physmat _hitactor) (`GameplayStatics.BreakHitResult` _outhit))
    (if _bblockinghit
      (if (> (`KismetArrayLibrary.Array_Length` (`CCharacterController.ItemsRightHand` _ccharactercontroller)) 0)
        _
        (elif (`self.ActorHasTag` _hitactor "PickUpable")
          (bind _ascgame_object (cast `CGameObject` _hitactor))
          (`CCharacterController.OnPickUp` _ccharactercontroller _ascgame_object)
          (message `/Game/Objects/IGameObject.OnPickUp` _ascgame_object (`self.Mesh`)))))))

(event `EnhancedInput|/Game/Input/PlayerThrowDown`
  (params (ActionValue :type Boolean) (ElapsedSeconds :type "Float (double-precision)") (TriggeredSeconds :type "Float (double-precision)") (InputAction :type "InputAction Object Reference" :default "/Game/Input/PlayerThrowDown.PlayerThrowDown"))
  (:`Triggered`
    (if (> (`KismetArrayLibrary.Array_Length` (`CCharacterController.ItemsRightHand` (`self.CCharacterController`))) 0)
      (for _array_element _
        (message `/Game/Objects/IGameObject.OnThrowDown` _array_element true)
        (bind _ascgame_object (cast `CGameObject` _array_element))
        (`CCharacterController.OnThrowDown` (`self.CCharacterController`) _ascgame_object)
        (set `self.DynamicMesh` null)))))

(event `EnhancedInput|/Game/Input/PlayerPlaceObject`
  (params (ActionValue :type Boolean) (ElapsedSeconds :type "Float (double-precision)") (TriggeredSeconds :type "Float (double-precision)") (InputAction :type "InputAction Object Reference" :default "/Game/Input/PlayerPlaceObject.PlayerPlaceObject"))
  (bind _dynamicmesh (`self.DynamicMesh`))
  (bind _dynamicmesh_2 (`self.DynamicMesh`))
  (bind _staticmesh (`/Game/Objects/DynamicMesh.StaticMesh` _dynamicmesh))
  (bind _returnvalue (`SceneComponent.K2_GetComponentToWorld` (`/Game/Objects/DynamicMesh.StaticMesh` _dynamicmesh_2)))
  (:`Started`
    (bind (_length _array) (`self.GetRightHandSize`))
    (if (> _length 0)
      (bind _mesh (`CGameObject.Mesh` (`|GetArrayItem` _array)))
      (bind _returnvalue_2 (`|SpawnActorFromClass` "/Game/Objects/DynamicMesh.DynamicMesh_C" (`KismetMathLibrary.MakeTransform` (+ (`self.K2_GetActorLocation`) (* (`SceneComponent.GetForwardVector` (`self.Camera`)) 400.0)) (struct) (`SceneComponent.K2_GetComponentScale` _mesh)) "AdjustIfPossibleButAlwaysSpawn" "MultiplyWithRoot" null null))
      (bind _output_get (set `self.DynamicMesh` _returnvalue_2))
      (bind _staticmesh_2 (`/Game/Objects/DynamicMesh.StaticMesh` _output_get))
      (`StaticMeshComponent.SetStaticMesh` _staticmesh_2 (`StaticMeshComponent.StaticMesh` _mesh))
      (`PrimitiveComponent.SetMaterial` _staticmesh_2 0 "/Game/Materials/ShapeMat.ShapeMat")
      (`PrimitiveComponent.SetCollisionEnabled` _staticmesh_2 "QueryOnly")
      (`SceneComponent.SetWorldScale3D` _staticmesh_2 (`SceneComponent.RelativeScale3D` _mesh))
      (`PrimitiveComponent.SetSimulatePhysics` _staticmesh true)
      (`PhysicsHandleComponent.GrabComponentAtLocation` (`/Game/Objects/DynamicMesh.PhysicsHandle` _dynamicmesh) _staticmesh "None" (`self.K2_GetActorLocation` _dynamicmesh))))
  (:`Completed`
    (bind (_length_2 _array_2) (`self.GetRightHandSize`))
    (if (> _length_2 0)
      (bind _output (`|GetArrayItem` _array_2))
      (message `/Game/Objects/IGameObject.OnThrowDown` _output true)
      (`SceneComponent.K2_SetWorldTransform` (`Actor.RootComponent` _output) _returnvalue false false)
      (bind _mesh_2 (`CGameObject.Mesh` _output))
      (`SceneComponent.K2_SetWorldTransform` _mesh_2 _returnvalue false false)
      (message `/Game/Objects/IGameObject.UpdateMeshLocation` _mesh_2)
      (`PhysicsHandleComponent.ReleaseComponent` (`/Game/Objects/DynamicMesh.PhysicsHandle` _dynamicmesh_2))
      (`CCharacterController.OnThrowDown` (`self.CCharacterController`) _output)
      (`self.K2_DestroyActor` _dynamicmesh_2)
      (set `self.DynamicMesh` null))))

(event `EnhancedInput|/Game/Input/PlayerObjectRotation`
  (params (ActionValue :type Boolean) (ElapsedSeconds :type "Float (double-precision)") (TriggeredSeconds :type "Float (double-precision)") (InputAction :type "InputAction Object Reference" :default "/Game/Input/PlayerObjectRotation.PlayerObjectRotation"))
  (bind _dynamicmesh (`self.DynamicMesh`))
  (bind _staticmesh (`/Game/Objects/DynamicMesh.StaticMesh` _dynamicmesh))
  (:`Triggered`
    (`/Engine/EditorBlueprintResources/StandardMacros.IsValid` _dynamicmesh
      (:`Is Valid`
        (if (`self.IsShiftActive`)
          (`SceneComponent.K2_AddWorldRotation` _staticmesh (`KismetMathLibrary.MakeRotator` 10.0) false false)
          (elif (`self.IsStrgActive`)
            (`SceneComponent.K2_AddWorldRotation` _staticmesh (`KismetMathLibrary.MakeRotator` 0.0 0.0 10.0) false false)
            (else
              (`SceneComponent.K2_AddWorldRotation` _staticmesh (`KismetMathLibrary.MakeRotator` 0.0 10.0) false false))))
        (`self.K2_SetActorRotation` _dynamicmesh (`SceneComponent.K2_GetComponentRotation` _staticmesh) false)))))

(event `self.ReceiveTick`
  (params (DeltaSeconds :type "Float (single-precision)"))
  (bind _camera (`self.Camera`))
  (bind _dynamicmesh (`self.DynamicMesh`))
  (`/Engine/EditorBlueprintResources/StandardMacros.IsValid` _dynamicmesh
    (:`Is Valid`
      (`PhysicsHandleComponent.SetTargetLocation` (`/Game/Objects/DynamicMesh.PhysicsHandle` _dynamicmesh) (+ (`SceneComponent.K2_GetComponentLocation` _camera) (* (`SceneComponent.GetForwardVector` _camera) 300.0))))))

(event `EnhancedInput|/Game/Input/PlayerPunch`
  (params (ActionValue :type Boolean) (ElapsedSeconds :type "Float (double-precision)") (TriggeredSeconds :type "Float (double-precision)") (InputAction :type "InputAction Object Reference" :default "/Game/Input/PlayerPunch.PlayerPunch"))
  (bind _rightpunchcollision (`self.RightPunchCollision`))
  (:`Triggered`
    (if (and (not (`NavMovementComponent.IsFalling` (`self.CharacterMovement`))) (not (`self.IsPunchActive`)))
      (set `self.IsPunchActive` true)
      (`PrimitiveComponent.SetCollisionEnabled` _rightpunchcollision "QueryAndPhysics")
      (`SkeletalMeshComponent.PlayAnimation` (`self.Mesh`) "/Game/ControlRig/Characters/Mannequins/Animations/Manny/MM_Punch.MM_Punch" false)
      (`KismetSystemLibrary.Delay` 2.0)
      (set `self.IsPunchActive` false)
      (`PrimitiveComponent.SetCollisionEnabled` _rightpunchcollision "NoCollision"))))

(fn `GetRightHandSize`
  (returns (Length :type Integer) (Array :type "Array of CGameObject Object Reference"))
  (bind _itemsrighthand (`CCharacterController.ItemsRightHand` (`self.CCharacterController`)))
  (return (`KismetArrayLibrary.Array_Length` _itemsrighthand) _itemsrighthand))

(fn `UserConstructionScript`)
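; BP_RaspberryBush08 is a raspberry bush environment actor that grows over time and resets when punched.
; Each tick, PlantGrowth adds growth scaled by GrowthRate until it reaches a threshold and marks the bush mature.
; Overlap with an actor tagged PunchCollider calls OnHarvest, which clears maturity and growth without checking maturity or granting any item.
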(event `self.ReceiveTick`
  (params (DeltaSeconds :type "Float (single-precision)"))
  (`self.PlantGrowth` DeltaSeconds))

(event `self.ReceiveActorBeginOverlap`
  (params (OtherActor :type "Actor Object Reference"))
  (if (`self.ActorHasTag` OtherActor "PunchCollider")
    (`self.OnHarvest`)))

(fn `OnHarvest`
  (set `self.IsMature` false)
  (set `self.CurrentGrowth` 0.0))

(fn `PlantGrowth`
  (params (DeltaTime :type "Float (double-precision)"))
  (if (not (`self.IsMature`))
    (bind _output_get (set `self.CurrentGrowth` (+ (* DeltaTime (`self.GrowthRate`)) (`self.CurrentGrowth`))))
    (if (>= _output_get 100.0)
      (set `self.IsMature` true))))

(fn `UserConstructionScript`)
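; BP_TreeSingleTrunk is an environment tree actor with a single trunk, built on a parent class whose construction script it calls.
; On BeginPlay it assigns its Trunk to the Mesh variable.
; Its Hit event checks for the Villager tag and, when the tree is a child actor, casts the parent actor to BP_GameObject, with no action after the cast.
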(event `self.ReceiveBeginPlay`
  (set `self.Mesh` (`self.Trunk`)))

(event `self.ReceiveHit`
  (params (MyComp :type "PrimitiveComponent Object Reference") (Other :type "Actor Object Reference") (OtherComp :type "PrimitiveComponent Object Reference") (bSelfMoved :type Boolean) (HitLocation :type "Vector Structure") (HitNormal :type "Vector Structure") (NormalImpulse :type "Vector Structure") (Hit :type "HitResult Structure (by ref)"))
  (if (`self.ActorHasTag` Other "Villager")
    (if (`self.IsChildActor` self)
      (cast `/Game/Objects/BP_GameObject` (`self.GetParentActor` self)))))

(fn `UserConstructionScript`
  (`parent.UserConstructionScript`))
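; BP_FullTree is a standing tree that villagers can fell by hitting it.
; BeginPlay sets its mesh, and each hit from an actor tagged Villager calls OnHit, then checks Durability.
; At zero durability it swaps itself for separate trunk and lowered stump actors, then applies a force to the trunk against the hit normal.
; A debug print shows that force.
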(event `self.ReceiveBeginPlay`
  (set `self.Mesh` (`self.FullTree`)))

(event `self.ReceiveHit`
  (params (MyComp :type "PrimitiveComponent Object Reference") (Other :type "Actor Object Reference") (OtherComp :type "PrimitiveComponent Object Reference") (bSelfMoved :type Boolean) (HitLocation :type "Vector Structure") (HitNormal :type "Vector Structure") (NormalImpulse :type "Vector Structure") (Hit :type "HitResult Structure (by ref)"))
  (bind _returnvalue (* HitNormal -10000.0))
  (bind _rotation (.rotation (`self.GetTransform`)))
  (bind (_x _y _z) (`KismetMathLibrary.BreakVector3f` (.location (`self.GetTransform`))))
  (if (`self.ActorHasTag` Other "Villager")
    (`self.OnHit` self 0)
    (if (<= (`self.Durability`) 0)
      (bind _returnvalue_2 (`|SpawnActorFromClass` "/Game/Environment/BP_TreeFullTrunk.BP_TreeFullTrunk_C" (`KismetMathLibrary.MakeTransform` (`KismetMathLibrary.MakeVector` _x _y _z) _rotation) "Undefined" "OverrideRootScale" null null))
      (`|SpawnActorFromClass` "/Game/Environment/BP_TreeStump.BP_TreeStump_C" (`KismetMathLibrary.MakeTransform` (`KismetMathLibrary.MakeVector` _x _y (- _z 337.5)) _rotation) "Undefined" "OverrideRootScale" null null)
      (`self.K2_DestroyActor`)
      (`PrimitiveComponent.AddForce` (`/Game/Environment/BP_TreeFullTrunk.Trunk` _returnvalue_2) _returnvalue "None" false)
      (`KismetSystemLibrary.PrintString` (`KismetStringLibrary.Conv_VectorToString` _returnvalue)))))

(fn `UserConstructionScript`
  (`parent.UserConstructionScript`))
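; BP_EnvironmentSpawner scatters randomly chosen environment objects around itself when play begins.
; A BeginPlay loop spawns actors up to MaxObjectsToSpawn, taking each class from a random SpawnableObjects entry; the Length-1 random bound never selects the last one.
; X and Y are random offsets from the spawner's location, while Z is an absolute random height, as the actor-relative Z calculation is left unconnected.
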(event `self.ReceiveBeginPlay`
  (bind _spawnableobjects (`self.SpawnableObjects`))
  (bind _maxobjectstospawn (`self.MaxObjectsToSpawn`))
  (bind _objectsspawned (`self.ObjectsSpawned`))
  ;[1 1 1] In C++
  (for _ (range (+ _maxobjectstospawn 1))
    (if (not (>= _objectsspawned _maxobjectstospawn))
      (`/Engine/EditorBlueprintResources/StandardMacros.IncrementInt` _objectsspawned
        (:`  `
          (`|SpawnActorFromClass` (`GameplayStatics.GetObjectClass` (`|GetArrayItem` _spawnableobjects (`KismetMathLibrary.RandomInteger` (- (`KismetArrayLibrary.Array_Length` _spawnableobjects) 1)))) (`KismetMathLibrary.MakeTransform` (`KismetMathLibrary.MakeVector` (+ (.x (`self.K2_GetActorLocation`)) (`KismetMathLibrary.RandomFloatInRange` (`self.MinRandomPositionX`) (`self.MaxRandomPositionX`))) (+ (.y (`self.K2_GetActorLocation`)) (`KismetMathLibrary.RandomFloatInRange` (`self.MinRandomPositionY`) (`self.MaxRandomPositionY`))) (`KismetMathLibrary.RandomFloatInRange` (`self.MinRandomPositionZ`) (`self.MaxRandomPositionZ`)))) "Undefined" "MultiplyWithRoot" null null))))))

(fn `UserConstructionScript`)
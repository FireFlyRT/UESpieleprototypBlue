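; BP_Observer is the observer's controlled Blueprint, letting the player show the mouse cursor while the Alt input is active.
; On BeginPlay it adds the ObserverInput Enhanced Input mapping context to its player controller.
; AltInput Triggered and Completed events set an IsAltActivated flag, which Tick copies every frame to player 0's cursor visibility.
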(event `self.ReceiveBeginPlay`
  (set `self.IsAltActivated` false)
  (bind _asplayer_controller (cast `PlayerController` (`self.GetController`)))
  (message `EnhancedInputSubsystemInterface.AddMappingContext` (pcsubsystem `EnhancedInputLocalPlayerSubsystem` _asplayer_controller) "/Game/Input/ObserverInput.ObserverInput" 0 (struct)))

(event `self.ReceiveTick`
  (params (DeltaSeconds :type "Float (single-precision)"))
  (set `PlayerController.bShowMouseCursor` (`self.IsAltActivated`) (`GameplayStatics.GetPlayerController` 0)))

(event `EnhancedInput|/Game/Input/AltInput`
  (params (ActionValue :type "Float (double-precision)") (ElapsedSeconds :type "Float (double-precision)") (TriggeredSeconds :type "Float (double-precision)") (InputAction :type "InputAction Object Reference" :default "/Game/Input/AltInput.AltInput"))
  (:`Triggered`
    (set `self.IsAltActivated` (> ActionValue 0.0) :!label _label))
  (:`Completed`
    (goto _label)))

(fn `UserConstructionScript`)
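; BP_GameObject is an actor for a physical game object that can be picked up and put down.
; OnPickUp disables mesh physics and collision, takes the carrier's owner and snaps to the HendHeldBoth socket.
; While attached, Tick moves the mesh to the scene root's world location each frame.
; OnThrowDown detaches it, restores collision, optionally re-enables physics and makes the object its own owner.
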(event `/Game/Objects/IGameObject.OnPickUp`
  (params (Parent :type "SkeletalMeshComponent Object Reference"))
  (bind _mesh (`self.Mesh`))
  (`self.K2_DetachFromActor` "KeepRelative")
  (`PrimitiveComponent.SetSimulatePhysics` _mesh false)
  (`PrimitiveComponent.WakeAllRigidBodies` _mesh)
  (`PrimitiveComponent.SetCollisionEnabled` _mesh "NoCollision")
  (`self.SetOwner` (`ActorComponent.GetOwner` Parent))
  (`self.K2_AttachToComponent` Parent "HendHeldBoth" "SnapToTarget" "SnapToTarget" "SnapToTarget")
  (set `self.IsAttached` true))

(event `/Game/Objects/IGameObject.OnThrowDown`
  (params (EnablePhysics :type Boolean))
  (bind _mesh (`self.Mesh`))
  (set `self.IsAttached` false)
  (`self.K2_DetachFromActor` "KeepRelative")
  (if EnablePhysics
    (`PrimitiveComponent.SetSimulatePhysics` _mesh true))
  (`PrimitiveComponent.WakeAllRigidBodies` _mesh)
  (`PrimitiveComponent.SetCollisionEnabled` _mesh "QueryAndPhysics")
  (`self.SetOwner` self))

(event `self.ReceiveTick`
  (params (DeltaSeconds :type "Float (single-precision)"))
  (if (`self.IsAttached`)
    (`/Game/Objects/IGameObject.UpdateMeshLocation`)))

(event `/Game/Objects/IGameObject.UpdateMeshLocation`
  (`SceneComponent.K2_SetWorldLocation` (`self.Mesh`) (`SceneComponent.K2_GetComponentLocation` (`self.DefaultSceneRoot`)) false false))

(fn `UserConstructionScript`)